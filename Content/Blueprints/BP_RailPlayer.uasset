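; BP_RailPlayer is a player Blueprint for rail-based movement with shooting.
; On BeginPlay it passes the spline component from SplinePathActor to its RailMovement component.
; Each Tick polls the first player controller for a left mouse press, then calls Fire on Shooting and plays shot effects through ShootingVisuals.
; Movement, firing logic and visuals are delegated to those separate components.
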(event EventBeginPlay
  (Class|RailMovementComponent|SetSpline (Variables|Default|GetRailMovement) (Actor|GetComponentbyClass (Variables|Default|GetSplinePathActor) "/Script/Engine.SplineComponent")))

(event EventTick
  (params (DeltaSeconds :type Float%20%28single-precision%29))
  (if (Game|Player|WasInputKeyJustPressed (Game|GetPlayerController 0) "LeftMouseButton")
    (Class|ShootingComponent|Fire (Variables|Default|GetShooting))
    (Class|ShootingVisualsComponent|PlayShotVisuals (Variables|Default|GetShootingVisuals))))

(fn ConstructionScript)